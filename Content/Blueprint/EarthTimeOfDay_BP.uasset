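; Earth time-of-day controller that scrubs the lighting cycle forward while Y is held and backward while U is held.
; BeginPlay seeks parallel timelines to StartTOD; their updates follow TODSpeed and drive sun rotation, temperature, intensity, disc scale, atmospheric and height fog, and skylight intensity.
; The sun timeline writes the current time back into StartTOD.
; A WIP Tick check recaptures the skylight when StartTOD exactly equals one of four set times.
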(event `Key|Y`
  (params (Key :type "Key Structure"))
  ;[1 1 1] Time of day control
  (:`Pressed`
    (set `self.TOD Speed` 200.0))
  (:`Released`
    (set `self.TOD Speed` 0.0 :!label _label)))

(event `Key|U`
  (params (Key :type "Key Structure"))
  ;[1 1 1] Time of day control
  (:`Pressed`
    (set `self.TOD Speed` -200.0))
  (:`Released`
    (goto _label)))

(event `self.ReceiveBeginPlay`
  (`|ExecutionSequence`
    (:`then_0`
      ;[1 1 1] Time of day control
      (bind (_direction _sunpitch _sunyaw _timeofday) (`Timeline|SunMovementTL` :`NewTime` (`self.StartTOD`) :!via `SetNewTime`)
        (:`Update`
          (`TimelineComponent.SetPlayRate` (`self.SunMovementTL`) (`self.TOD Speed`))
          (`self.K2_SetActorRotation` (`self.DirectionalLight`) (`KismetMathLibrary.MakeRotator` 0.0 _sunpitch _sunyaw) false)
          (set `self.StartTOD` _timeofday))))
    (:`then_1`
      ;[1 1 1] Temperature TOD
      (bind (_direction_2 _temperature) (`Timeline|TemperatureTL` :`NewTime` (`self.StartTOD`) :!via `SetNewTime`)
        (:`Update`
          (`TimelineComponent.SetPlayRate` (`self.TemperatureTL`) (`self.TOD Speed`))
          (`LightComponent.SetTemperature` (`Light.LightComponent` (`self.DirectionalLight`)) _temperature))))
    (:`then_2`
      ;[1 1 1] Sun intensity TOD
      (bind (_direction_3 _sunintensity) (`Timeline|SunIntensityTL` :`NewTime` (`self.StartTOD`) :!via `SetNewTime`)
        (:`Update`
          (`TimelineComponent.SetPlayRate` (`self.SunIntensityTL`) (`self.TOD Speed`))
          (`LightComponent.SetIntensity` (`Light.LightComponent` (`self.DirectionalLight`)) _sunintensity))))
    (:`then_3`
      ;[1 1 1] Atmospheric fog sun multiplier TOD
      (bind (_direction_4 _sunmultiplier) (`Timeline|AtmosphericFogSunMultiplierTL` :`NewTime` (`self.StartTOD`) :!via `SetNewTime`)
        (:`Update`
          (`TimelineComponent.SetPlayRate` (`self.AtmosphericFogSunMultiplierTL`) (`self.TOD Speed`))
          (`AtmosphericFogComponent.SetSunMultiplier` (`AtmosphericFog.AtmosphericFogComponent` (`self.AtmosphericFog`)) _sunmultiplier))))
    (:`then_4`
      ;[1 1 1] Exponential fog density TOD
      (bind (_direction_5 _fogdensity) (`Timeline|ExponentialFogDensityTL` :`NewTime` (`self.StartTOD`) :!via `SetNewTime`)
        (:`Update`
          (`TimelineComponent.SetPlayRate` (`self.ExponentialFogDensityTL`) (`self.TOD Speed`))
          (`ExponentialHeightFogComponent.SetFogDensity` (`ExponentialHeightFog.Component` (`self.ExponentialHeightFog`)) _fogdensity))))
    (:`then_5`
      ;[1 1 1] Sun disc scale TOD
      (bind (_direction_6 _sundiscscale) (`Timeline|SunDiscScaleTL` :`NewTime` (`self.StartTOD`) :!via `SetNewTime`)
        (:`Update`
          (`TimelineComponent.SetPlayRate` (`self.SunDiscScaleTL`) (`self.TOD Speed`))
          (set `AtmosphericFogComponent.SunDiscScale` _sundiscscale (`AtmosphericFog.AtmosphericFogComponent` (`self.AtmosphericFog`))))))
    (:`then_6`
      ;[1 1 1] Atmospheric fog sun multiplier TOD
      (bind (_direction_7 _fogdensity_2) (`Timeline|AtmosphericFogDensityTL` :`NewTime` (`self.StartTOD`) :!via `SetNewTime`)
        (:`Update`
          (`TimelineComponent.SetPlayRate` (`self.AtmosphericFogDensityTL`) (`self.TOD Speed`))
          (`AtmosphericFogComponent.SetDensityMultiplier` (`AtmosphericFog.AtmosphericFogComponent` (`self.AtmosphericFog`)) _fogdensity_2))))
    (:`then_7`
      ;[1 1 1] Skylight TOD
      (bind (_direction_8 _skylightintensity) (`Timeline|SkyLightTL` :`NewTime` (`self.StartTOD`) :!via `SetNewTime`)
        (:`Update`
          (`TimelineComponent.SetPlayRate` (`self.SkyLightTL`) (`self.TOD Speed`))
          (`SkyLightComponent.SetIntensity` (`SkyLight.LightComponent` (`self.SkyLight`)) _skylightintensity))))))

(event `self.ReceiveTick`
  (params (DeltaSeconds :type "Float (single-precision)"))
  (bind _starttod (`self.StartTOD`))
  ;[1 1 1] Skylight Capture (WIP)
  (`|ExecutionSequence`
    (:`then_0`
      (if (== _starttod 800.0)
        (`SkyLightComponent.RecaptureSky` (`SkyLight.LightComponent` (`self.SkyLight`)) :!label _label_2)))
    (:`then_1`
      (if (== _starttod 1200.0)
        (goto _label_2)))
    (:`then_2`
      (if (== _starttod 1900.0)
        (goto _label_2)))
    (:`then_3`
      (if (== _starttod 2400.0)
        (goto _label_2)))))

(fn `UserConstructionScript`)